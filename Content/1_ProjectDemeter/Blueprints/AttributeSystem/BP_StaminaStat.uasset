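; Stamina stat component for BP_BaseCharacter that links character movement to stamina logic.
; On BeginPlay it casts its owner and, only with authority, binds to gait, jump and roll events plus its own stamina-depleted delegate.
; ALS gait values are converted to walk, run or sprint for OnGaitUpdate, and depletion calls StopSprintOverride on the character.
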(event `self.ReceiveBeginPlay`
  (`self.Initalize`))

(event `Initalize`
  (bind _my_base_character (`self.My Base Character`))
  ;[1 1 1] Initalize
  (bind _asbp_base_character (cast `/Game/1_ProjectDemeter/Blueprints/CharacterSystem/BP_BaseCharacter` (`self.GetOwner`)))
  (bind _output_get (set `self.My Base Character` _asbp_base_character))
  (if (`Actor.HasAuthority` _output_get)
    (add `/Game/1_ProjectDemeter/Blueprints/CharacterSystem/BP_BaseCharacter.On Gait Updated` _my_base_character (`|CreateDelegate` :!event `Convert ALS Gait Enum`))
    (add `/Game/1_ProjectDemeter/Blueprints/CharacterSystem/BP_BaseCharacter.On Jump` _my_base_character (`|CreateDelegate` :!event `OnJump`))
    (add `/Game/1_ProjectDemeter/Blueprints/CharacterSystem/BP_BaseCharacter.On Roll` _my_base_character (`|CreateDelegate` :!event `OnRoll`))
    (add `self.OnStaminaDepletedChangeDelegate` (`|CreateDelegate` :!event `On Stamina Depleted Changed`))))

(fn `Convert ALS Gait Enum`
  (params (`New Gait` :type "/Game/Z_AdvancedLocomotionV4/Data/Enums/ALS_Gait Enum" :default "NewEnumerator0"))
  (`self.OnGaitUpdate` (select `/Game/Z_AdvancedLocomotionV4/Data/Enums/ALS_Gait` `New Gait` :`NewEnumerator0` "EG_Walk" :`NewEnumerator1` "EG_Run" :`NewEnumerator2` "EG_Sprint" :!type "EGait_New Enum")))

(fn `On Stamina Depleted Changed`
  (params (bIsDepleted :type Boolean))
  (if bIsDepleted
    (`/Game/1_ProjectDemeter/Blueprints/CharacterSystem/BP_BaseCharacter.Stop Sprint Override` (`self.My Base Character`))))