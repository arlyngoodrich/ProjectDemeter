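; Spline actor that spawns Niagara rain drips along its length, driven by Ultra Dynamic Weather.
; It samples the spline at intervals, traces downward for drop death heights and creates one emitter per segment.
; Straight runs with linearly varying collision heights collapse into a single emitter.
; Weather collection parameters update spawn rate, activation, splashes and wind-scaled curl noise on tick, unless the actor is set to ignore weather state.
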(event `/Game/Environment/WeatherSystem/Blueprints/Weather_Effects/Weather_Effects_Interface.Editor Update`
  (`self.Update with Weather`))

(event `self.ReceiveBeginPlay`
  (set `self.Runtime` true)
  (`self.Create Curve Data`)
  (`self.Update with Weather`)
  (if (not (`self.Ignore Weather State`))
    (`KismetSystemLibrary.Delay` (`KismetMathLibrary.RandomFloatInRange` 0.0 3.0))
    (`self.SetActorTickEnabled` true)))

(event `self.ReceiveTick`
  (params (DeltaSeconds :type "Float (single-precision)"))
  (`self.Update with Weather`))

(event `/Game/Environment/WeatherSystem/Blueprints/Weather_Effects/Weather_Effects_Interface.Reset Emitters`
  (`KismetSystemLibrary.Delay` 0.05)
  (`self.Update with Weather`)
  (`NiagaraComponent.ReinitializeSystem` (`self.Drip_Systems`)))

(fn `Check for Straight Line`
  (returns (Straight :type Boolean))
  (locals (`First Point` :type "Vector Structure") (`Last Point` :type "Vector Structure") (`Found Deviation` :type Boolean) (`Start Height` :type "Float (double-precision)") (`Last Height` :type "Float (double-precision)"))
  (bind _positions_array (`self.Positions Array`))
  (bind _death_heights_array (`self.Death Heights Array`))
  (set `local.First Point` (`|GetArrayItem` (`self.Positions Array`)))
  (set `local.Last Point` (`|GetArrayItem` _positions_array (`KismetArrayLibrary.Array_LastIndex` _positions_array)))
  (for _array_element (`self.Positions Array`)
    (if (> (`KismetMathLibrary.GetPointDistanceToSegment` _array_element (`local.First Point`) (`local.Last Point`)) (/ (`self.Point Spacing`) 10.0))
      (set `local.Found Deviation` true)
      (break)))
  (if (not (`local.Found Deviation`))
    (set `local.Start Height` (`|GetArrayItem` (`self.Death Heights Array`)))
    (set `local.Last Height` (`|GetArrayItem` _death_heights_array (`KismetArrayLibrary.Array_LastIndex` _death_heights_array)))
    (for (_array_element_2 _array_index) (`self.Death Heights Array`)
      (if (> (`KismetMathLibrary.Abs` (- _array_element_2 (`KismetMathLibrary.MapRangeClamped` (`KismetMathLibrary.Conv_IntToDouble` _array_index) 0.0 (`KismetMathLibrary.Conv_IntToDouble` (`KismetArrayLibrary.Array_LastIndex` (`self.Death Heights Array`))) (`local.Start Height`) (`local.Last Height`)))) (/ (`self.Point Spacing`) 10.0))
        (set `local.Found Deviation` true)
        (break))))
  (return (not (`local.Found Deviation`))))

(fn `Create Curve Data`
  (locals (Total_Distance :type "Float (double-precision)" :default 0.0) (`Last Collision Index` :type Integer :default 0))
  (`ActorComponent.K2_DestroyComponent` (`self.Drip_Systems`))
  (`KismetArrayLibrary.Array_Clear` (`self.Drip_Systems`))
  (set `local.Total_Distance` (`SplineComponent.GetSplineLength` (`self.Spline`)))
  (`KismetArrayLibrary.Array_Clear` (`self.Death Heights Array`))
  (`KismetArrayLibrary.Array_Clear` (`self.Positions Array`))
  (bind _output_get (set `local.Last Collision Index` (`KismetMathLibrary.Clamp` (`KismetMathLibrary.FCeil` (/ (`local.Total_Distance`) (`self.Point Spacing`))) 1 1000)))
  (for _index (range (+ _output_get 1))
    (bind _returnvalue (`SplineComponent.GetLocationAtDistanceAlongSpline` (`self.Spline`) (`KismetMathLibrary.MapRangeClamped` (`KismetMathLibrary.Conv_IntToDouble` _index) 0.0 (`KismetMathLibrary.Conv_IntToDouble` (`local.Last Collision Index`)) 0.0 (`local.Total_Distance`)) "World"))
    (`KismetArrayLibrary.Array_Add` (`self.Positions Array`) _returnvalue)
    (bind _returnvalue_2 (- _returnvalue (0.0 0.0 10000.0)))
    (bind (_outhit _returnvalue_3) (`KismetSystemLibrary.LineTraceSingle` (- _returnvalue (`KismetMathLibrary.MakeVector` 0.0 0.0 (`self.Collision Line Trace Head Start`))) _returnvalue_2 (`self.Collision Trace Channel`) false (`self.Collision Actors to Ignore`) (select `bool` (`self.Runtime`) :`false` "ForDuration" :!type "EDrawDebugTrace Enum") true (struct :`R` 0.194618 :`G` 0.327778 :`B` 0.462077 :`A` 1.0) (struct :`A` 1.0) 0.1))
    (if _returnvalue_3
      (`KismetArrayLibrary.Array_Add` (`self.Death Heights Array`) (.z (`.Location` (`GameplayStatics.BreakHitResult` _outhit))))
      (else
        (`KismetArrayLibrary.Array_Add` (`self.Death Heights Array`) (.z _returnvalue_2)))))
  (if (not (`KismetArrayLibrary.Array_IsValidIndex` (`self.Drip_Systems`)))
    (bind _straight (`self.Check for Straight Line`))
    (bind _output_get_2 (set `self.Straight Line` _straight))
    (if _output_get_2
      (for _ (range (+ (- (`local.Last Collision Index`) 2) 1))
        (if (`KismetArrayLibrary.Array_IsValidIndex` (`self.Positions Array`) 1)
          (`KismetArrayLibrary.Array_Remove` (`self.Positions Array`) 1)
          (`KismetArrayLibrary.Array_Remove` (`self.Death Heights Array`) 1))))
    (for (_array_element _array_index) (`self.Positions Array`)
      (bind _returnvalue_4 (+ _array_index 1))
      (if (`KismetArrayLibrary.Array_IsValidIndex` (`self.Positions Array`) _returnvalue_4)
        (bind _returnvalue_5 (`AddComponent|NODE_AddNiagaraComponent-0` :`RelativeTransform` (`KismetMathLibrary.MakeRelativeTransform` (`KismetMathLibrary.MakeTransform` _array_element) (`self.GetTransform`))))
        (`KismetArrayLibrary.Array_Add` (`self.Drip_Systems`) _returnvalue_5)
        (`FXSystemComponent.SetVectorParameter` _returnvalue_5 "Line End" (`|GetArrayItem` (`self.Positions Array`) _returnvalue_4))
        (`FXSystemComponent.SetFloatParameter` _returnvalue_5 "Start_Death Height" (`|GetArrayItem` (`self.Death Heights Array`) (- _returnvalue_4 1)))
        (`FXSystemComponent.SetFloatParameter` _returnvalue_5 "End_Death Height" (`|GetArrayItem` (`self.Death Heights Array`) _returnvalue_4))))))

(fn `Update with Weather`
  (locals (Raining :type "Float (double-precision)" :default 0.0))
  (bind _current_spawn_rate (`self.Current Spawn Rate`))
  (bind _returnvalue (`KismetMaterialLibrary.GetScalarParameterValue` "/Game/Environment/WeatherSystem/Materials/Weather/UltraDynamicWeather_Parameters.UltraDynamicWeather_Parameters" "Wet"))
  (bind _returnvalue_2 (`KismetMaterialLibrary.GetScalarParameterValue` "/Game/Environment/WeatherSystem/Materials/Weather/UltraDynamicWeather_Parameters.UltraDynamicWeather_Parameters" "Raining"))
  (set `local.Raining` (`KismetMathLibrary.SelectFloat` 1.0 _returnvalue_2 (`self.Ignore Weather State`)))
  (set `self.Current Spawn Rate` (* (`KismetMathLibrary.SelectFloat` 1.0 (`KismetMathLibrary.FClamp` (+ _returnvalue_2 (* _returnvalue 0.01))) (`self.Ignore Weather State`)) (+ (* (`self.Spawn Rate Per Meter`) (/ (/ (`SplineComponent.GetSplineLength` (`self.Spline`)) (`KismetMathLibrary.Conv_IntToDouble` (`KismetArrayLibrary.Array_Length` (`self.Drip_Systems`)))) 100.0)) (`self.Extra Spawn Rate`))))
  (for _array_element (`self.Drip_Systems`)
    (`FXSystemComponent.SetFloatParameter` _array_element "Spawn Rate" (`KismetMathLibrary.SelectFloat` _current_spawn_rate (* _current_spawn_rate (`KismetMathLibrary.RandomFloatInRange` 0.5 2.0)) (`self.Straight Line`))))
  (`|ExecutionSequence`
    (:`then_0`
      (bind _output_get (set `self.System Active` (> (`self.Current Spawn Rate`) 0.0)))
      (`ActorComponent.SetActive` (`self.Drip_Systems`) _output_get false))
    (:`then_1`
      (if (`self.System Active`)
        (bind _returnvalue_3 (`KismetMaterialLibrary.GetVectorParameterValue` "/Game/Environment/WeatherSystem/Materials/Weather/UltraDynamicWeather_Parameters.UltraDynamicWeather_Parameters" "Wind Force"))
        (`FXSystemComponent.SetFloatParameter` (`self.Drip_Systems`) "Curl Noise Force" (* (`KismetMathLibrary.MapRangeClamped` (`KismetMathLibrary.VSize` (`KismetMathLibrary.Conv_LinearColorToVector` _returnvalue_3)) 0.0 2000.0 42.0 140.0) (`self.Curl Noise Force`)))
        (`FXSystemComponent.SetIntParameter` (`self.Drip_Systems`) "Splash Duplicate Count" (`KismetMathLibrary.Round` (`KismetMathLibrary.MapRangeClamped` (`local.Raining`) 0.1 1.0 1.0 2.0)))
        (`FXSystemComponent.SetFloatParameter` (`self.Drip_Systems`) "Splash Duplicate Range" (`KismetMathLibrary.MapRangeClamped` (`local.Raining`) 0.0 1.0 0.0 6.0))))))

(fn `UserConstructionScript`
  (set `self.Refresh` false)
  (`self.Create Curve Data`)
  (`self.Update with Weather`)
  (`FXSystemComponent.SetFloatParameter` (`self.Drip_Systems`) "Splash Percentage" (`self.Splash Frequency`))
  (`FXSystemComponent.SetFloatParameter` (`self.Drip_Systems`) "Drop Scale" (`self.Drops Scale`)))