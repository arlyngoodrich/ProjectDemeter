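; Spline-bounded volume that overrides Ultra Dynamic Weather within a region, registering itself with the weather actor while it exists.
; Its weather values come from a fixed preset at BeginPlay or are copied each tick from a seasonal Random Weather Variation component.
; On authority, Tick schedules regional lightning flashes using a delay derived from those values.
; Construction closes the spline, scales points by transition width, and, outside packaged builds, precomputes sphere bounds and adds colored labels.
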(event `self.ReceiveBeginPlay`
  ;[0.5781 0.3561 1 1 45] Initialize Volume
  (bind _returnvalue (`GameplayStatics.GetActorOfClass` "/Game/Environment/WeatherSystem/Blueprints/Ultra_Dynamic_Weather.Ultra_Dynamic_Weather_C"))
  (`/Engine/EditorBlueprintResources/StandardMacros.IsValid` _returnvalue
    (:`Is Valid`
      (bind _output_get (set `self.UDW` _returnvalue))
      (`KismetArrayLibrary.Array_Add` (`/Game/Environment/WeatherSystem/Blueprints/Ultra_Dynamic_Weather.Weather Override Volumes` _output_get) self)
      (`/Game/Environment/WeatherSystem/Blueprints/Ultra_Dynamic_Weather.Sort Weather Override Volumes` (`self.UDW`))
      (switch `/Game/Environment/WeatherSystem/Blueprints/Enum/UDS_Weather_Override_Mode` (`self.Mode`)
        (:`NewEnumerator0`
          (bind (_weather_intensity _cloud_coverage _rain___snow _wind_intensity _material_wetness _material_snow) (`/Game/Environment/WeatherSystem/Blueprints/Ultra_Dynamic_Weather.Get Weather Preset` (`self.UDW`) (`self.Weather Type`)))
          (set `self.Weather Intensity` _weather_intensity)
          (set `self.Cloud Coverage` _cloud_coverage)
          (set `self.Rain / Snow` _rain___snow)
          (set `self.Wind Intensity` _wind_intensity)
          (set `self.Material Wetness` _material_wetness)
          (set `self.Material Snow` _material_snow))
        (:`NewEnumerator1`
          (`/Game/Environment/WeatherSystem/Blueprints/Weather_Effects/System/Random_Weather_Variation.Initialize` (`self.Random_Weather_Variation`) (`self.UDW`) (`self.Weather Type Probabilities (Summer)`) (`self.Weather Type Probabilities (Autumn)`) (`self.Weather Type Probabilities (Winter)`) (`self.Weather Type Probabilities (Spring)`) true))))))

(event `self.ReceiveDestroyed`
  ;[0.5781 0.3561 1 1 45] Initialize Volume
  (`KismetArrayLibrary.Array_RemoveItem` (`/Game/Environment/WeatherSystem/Blueprints/Ultra_Dynamic_Weather.Weather Override Volumes` (`self.UDW`)) self)
  (`/Game/Environment/WeatherSystem/Blueprints/Ultra_Dynamic_Weather.Sort Weather Override Volumes` (`self.UDW`)))

(event `self.ReceiveTick`
  (params (DeltaSeconds :type "Float (single-precision)"))
  (`|ExecutionSequence`
    (:`then_0`
      ;[0.4142 1 0.3172 1 45] Update Random Weather
      (if (`|EnumEquality` (`self.Mode`) "NewEnumerator1")
        (set `self.Weather Intensity` (`/Game/Environment/WeatherSystem/Blueprints/Weather_Effects/System/Random_Weather_Variation.Random Weather Intensity` (`self.Random_Weather_Variation`)))
        (set `self.Cloud Coverage` (`/Game/Environment/WeatherSystem/Blueprints/Weather_Effects/System/Random_Weather_Variation.Random Cloud Coverage` (`self.Random_Weather_Variation`)))
        (set `self.Wind Intensity` (`/Game/Environment/WeatherSystem/Blueprints/Weather_Effects/System/Random_Weather_Variation.Random Wind Intensity` (`self.Random_Weather_Variation`)))
        (set `self.Rain / Snow` (`/Game/Environment/WeatherSystem/Blueprints/Weather_Effects/System/Random_Weather_Variation.Random Rain / Snow` (`self.Random_Weather_Variation`)))
        (set `self.Material Snow` (`/Game/Environment/WeatherSystem/Blueprints/Weather_Effects/System/Random_Weather_Variation.Random Material Snow` (`self.Random_Weather_Variation`)))
        (set `self.Material Wetness` (`/Game/Environment/WeatherSystem/Blueprints/Weather_Effects/System/Random_Weather_Variation.Random Material Wetness` (`self.Random_Weather_Variation`)))))
    (:`then_1`
      ;[0.1514 0.3143 1 1 45] Spawn Lightning Flashes within Region
      (`/Engine/EditorBlueprintResources/ActorMacros.Switch Has Authority`
        (:`Authority`
          (bind _period (`/Game/Environment/WeatherSystem/Blueprints/Ultra_Dynamic_Weather.Current Lightning Period and Status` (`self.UDW`) (`self.Weather Intensity`) (`self.Cloud Coverage`) (`self.Rain / Snow`) false))
          (`KismetSystemLibrary.Delay` _period)
          (`/Game/Environment/WeatherSystem/Blueprints/Ultra_Dynamic_Weather.Flash Lightning Local` (`self.UDW`) self (`KismetMathLibrary.RandomFloatInRange` 0.0 360.0)))))))

(fn `Calculate Spline Bounds`
  (locals (Bounds :type "Float (double-precision)"))
  (bind _spline (`self.Spline`))
  (bind _returnvalue (* (`SplineComponent.GetNumberOfSplinePoints` _spline) 4))
  (for _index (range (+ _returnvalue 1))
    (bind _returnvalue_2 (`KismetMathLibrary.Vector_Distance` (`SplineComponent.GetLocationAtDistanceAlongSpline` (`self.Spline`) (* _index (/ (`SplineComponent.GetSplineLength` _spline) (`KismetMathLibrary.Conv_IntToDouble` _returnvalue))) "World") (`self.Spline Bounds Center`)))
    (if (> _returnvalue_2 (`local.Bounds`))
      (set `local.Bounds` _returnvalue_2)))
  (set `self.Total Sphere Bounds` (+ (`local.Bounds`) (/ (`self.Scaled Transition Width`) 1.8) 200.0)))

(fn `UserConstructionScript`
  (locals (Label :type String) (`Spline Points` :type "Array of Vector Structure") (`Text Component` :type "TextRenderComponent Object Reference"))
  (bind _spline (`self.Spline`))
  (bind _returnvalue (`SplineComponent.GetNumberOfSplinePoints` (`self.Spline`)))
  (bind _returnvalue_2 (`SplineComponent.GetSplineLength` (`self.Spline`)))
  (bind _returnvalue_3 (/ (`self.Scaled Transition Width`) 2.0))
  (bind _returnvalue_4 (`KismetMathLibrary.FFloor` (/ _returnvalue_2 (/ (`self.Total Sphere Bounds`) 3.5))))
  (set `self.Scaled Transition Width` (`self.Scale Transition Width`))
  ;[0.1472 1 0.1238 1 45] Analyze Spline and Set Scale of Points
  (for _index (range _returnvalue)
    (`SplineComponent.SetScaleAtSplinePoint` _spline _index (`KismetMathLibrary.MakeVector` _returnvalue_3 _returnvalue_3 _returnvalue_3) true)
    (`KismetArrayLibrary.Array_Add` (`local.Spline Points`) (`SplineComponent.GetLocationAtSplinePoint` _spline _index "World")))
  (`SplineComponent.SetClosedLoopAtPosition` (`self.Spline`) true (+ (`KismetMathLibrary.Conv_IntToDouble` _returnvalue) 0.001) true)
  ;[0.543 0.2454 1 1 45] Calculate and Save Bounds Information
  (if (not (`KismetSystemLibrary.IsPackagedForDistribution`))
    (set `self.Spline Bounds Center` (`KismetMathLibrary.GetVectorArrayAverage` (`local.Spline Points`)))
    (`self.Calculate Spline Bounds`)
    (set `/Game/Environment/WeatherSystem/Blueprints/Weather_Effects/System/Random_Weather_Variation.Volume` self (`self.Random_Weather_Variation`))
    ;[1 0.5038 0.1655 1 45] Weather Labels - Editor Only
    (`SplineComponent.SetUnselectedSplineSegmentColor` (`self.Spline`) (`self.Label Color`))
    (if (`self.Show Weather Label in Editor`)
      (set `local.Label` (select `/Game/Environment/WeatherSystem/Blueprints/Enum/UDS_Weather_Override_Mode` (`self.Mode`) :`NewEnumerator0` (`|GetEnumeratorNameAsString` (`self.Weather Type`)) :`NewEnumerator1` "Random"))
      (for _index_2 (range (+ _returnvalue_4 1))
        (bind _returnvalue_5 (`AddComponent|NODE_AddTextRenderComponent-2` :`RelativeTransform` (`KismetMathLibrary.MakeTransform` (.location (`SplineComponent.GetTransformAtDistanceAlongSpline` (`self.Spline`) (* _index_2 (/ _returnvalue_2 (`KismetMathLibrary.Conv_IntToDouble` _returnvalue_4))) "Local" false)) (`KismetMathLibrary.ComposeRotators` (.rotation (`SplineComponent.GetTransformAtDistanceAlongSpline` (`self.Spline`) (* _index_2 (/ _returnvalue_2 (`KismetMathLibrary.Conv_IntToDouble` _returnvalue_4))) "Local" false)) (struct :`Yaw` -90.0)) (/ (1.0 1.0 1.0) (`self.GetActorScale3D`)))))
        (set `local.Text Component` _returnvalue_5)
        (`TextRenderComponent.SetTextRenderColor` (`local.Text Component`) (`KismetMathLibrary.Conv_LinearColorToColor` (`self.Label Color`)))
        (`TextRenderComponent.SetWorldSize` (`local.Text Component`) (/ (`self.Total Sphere Bounds`) 20.0))
        (`TextRenderComponent.K2_SetText` (`local.Text Component`) (`KismetTextLibrary.Conv_StringToText` (`local.Label`)))))))