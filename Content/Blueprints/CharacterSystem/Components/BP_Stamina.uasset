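; Stamina component for BP_BaseCharacter that links the character's movement to inherited stamina logic.
; On BeginPlay it binds to the owner's gait, jump and roll events and forwards them, shifting gait by one to convert to EGait.
; When stamina depletes during one specific gait, it calls the character's sprint-stop override.
; Stamina events print optional debug messages, and DecreaseStamina is an empty stub.
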(event `self.ReceiveBeginPlay`
  (bind _my_base_character (`self.My Base Character`))
  (bind _asbp_base_character (cast `/Game/Blueprints/CharacterSystem/BP_BaseCharacter` (`self.GetOwner`)))
  (set `self.My Base Character` _asbp_base_character)
  (add `/Game/Blueprints/CharacterSystem/BP_BaseCharacter.On Gait Updated` _my_base_character (delegate `On Gait Updated`))
  (add `/Game/Blueprints/CharacterSystem/BP_BaseCharacter.On Jump` _my_base_character (delegate `Charter Jumped`))
  (add `/Game/Blueprints/CharacterSystem/BP_BaseCharacter.On Roll` _my_base_character (delegate `Character Rolled`)))

(event `On Gait Updated`
  (params (`New Gait` :type "/Game/Z_AdvancedLocomotionV4/Data/Enums/ALS_Gait Enum" :default "NewEnumerator0"))
  (bind _output_get (set `self.Current Gait` `New Gait`))
  (`self.OnGaitUpdate` (cast `EGait` (+ _output_get 1))))

(event `Charter Jumped`
  (`self.OnJump`))

(event `Character Rolled`
  (`self.OnRoll`))

(event `self.BP_OnStaminaDepleted`
  (`KismetSystemLibrary.PrintString` "Stamina Depleted" (`self.Debug Print`))
  (if (`|EnumEquality` (`self.Current Gait`) "NewEnumerator2")
    (`/Game/Blueprints/CharacterSystem/BP_BaseCharacter.Stop Sprint Override` (`self.My Base Character`))))

(event `self.BP_OnStaminaRegenerated`
  (`KismetSystemLibrary.PrintString` "Stamina Regenerated" (`self.Debug Print`)))

(event `self.BP_OnStaminaUpdate`
  (params (UpdatedStamina :type "Float (single-precision)"))
  (`KismetSystemLibrary.PrintString` (`KismetStringLibrary.Concat_StrStr` "Stamina: " (`KismetTextLibrary.Conv_TextToString` (`KismetTextLibrary.AsPercent_Float` (/ UpdatedStamina (`self.MaxStamina`)) "HalfToEven"))) (`self.Debug Print`)))

(fn `Decrease Stamina`)