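; BP_GoalTracking is a goal tracking component on BP_PlayerController that sets up test goals for the player.
; When the controller possesses a pawn, it adds a WBP_GoalDisplay widget for local controllers.
; With authority, it constructs, initializes and adds a chalice delivery goal targeting a BP_TestChest and a health potion pickup goal.
; A GoalsCreated flag, set only on the authority, guards against repeat creation.
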(event `self.ReceiveBeginPlay`
  (bind _asbp_player_controller (cast `/Game/Blueprints/Core/BP_PlayerController` (`self.GetOwner`)))
  (bind _output_get (set `self.Owning Controller` _asbp_player_controller))
  (add `/Game/Blueprints/Core/BP_PlayerController.On Possess` _output_get (delegate `Create Goal Test`)))

(event `Create Goal Test`
  (if (not (`self.Goals Created`))
    (if (`Controller.IsLocalController` (`self.Owning Controller`))
      (bind _returnvalue (`|CreateWidget` "/Game/Blueprints/GoalSystem/WBP_GoalDisplay.WBP_GoalDisplay_C" (`self.Owning Controller`) self))
      (`UserWidget.AddToViewport` _returnvalue 0))
    (if (`Actor.HasAuthority` (`self.GetOwner`))
      (bind _returnvalue_2 (`GameplayStatics.GetActorOfClass` "/Game/Debug/BP_TestChest.BP_TestChest_C"))
      (bind _returnvalue_3 (`|GenericCreateObject` "/Game/Debug/BP_DeliveryGoal.BP_DeliveryGoal_C" self _returnvalue_2 "/Game/Blueprints/ItemSystem/Items/Chalice/BP_Chalice.BP_Chalice_C" "Pickup Chalice" "Drop off Chalice"))
      (`GoalObjectBase.BP_Initialize` _returnvalue_3 (`self.Owning Controller`) self "Deliver Chalice" "Pickup Chalice for delivery")
      (`self.BP_AddGoal` _returnvalue_3)
      (bind _returnvalue_4 (`|GenericCreateObject` "/Game/Blueprints/GoalSystem/BP_PickupGoal.BP_PickupGoal_C" self "/Game/Blueprints/ItemSystem/Items/Potions/BP_HealthPotion.BP_HealthPotion_C"))
      (`GoalObjectBase.BP_Initialize` _returnvalue_4 (`self.Owning Controller`) self "Pickup Health Potion" "")
      (`self.BP_AddGoal` _returnvalue_4)
      (set `self.Goals Created` true))))