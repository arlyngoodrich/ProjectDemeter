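; BP_InteractableObject is an interaction component that highlights its owning actor while it has focus.
; On focus start, it enables Render Custom Depth on every mesh component of the owner and writes the OutlineStencil value to the custom depth stencil.
; On focus end, it disables custom depth on those meshes and sets the stencil to a fixed value.
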(event `self.BP_OnStartFocus`
  (for _array_element (`Actor.K2_GetComponentsByClass` (`self.GetOwner`) "/Script/Engine.MeshComponent")
    (`PrimitiveComponent.SetRenderCustomDepth` _array_element true)
    (`PrimitiveComponent.SetCustomDepthStencilValue` _array_element (`self.Outline Stencil`))))

(event `self.BP_OnEndFocus`
  (for _array_element (`Actor.K2_GetComponentsByClass` (`self.GetOwner`) "/Script/Engine.MeshComponent")
    (`PrimitiveComponent.SetRenderCustomDepth` _array_element false)
    (`PrimitiveComponent.SetCustomDepthStencilValue` _array_element 1)))